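; BP_Item is a material drop actor that the player can pick up into their inventory.
; Its Collision component's overlap events toggle InRange when a CH_Player enters or leaves.
; BeingPickedUp casts the instigator to PC_Player, adds ItemInformation to that player's Inventory, then destroys the actor.
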(event OnComponentBeginOverlap(Collision)
  (params (OverlappedComponent :type Primitive%20Component%20Object%20Reference) (OtherActor :type Actor%20Object%20Reference) (OtherComp :type Primitive%20Component%20Object%20Reference) (OtherBodyIndex :type Integer) (bFromSweep :type Boolean) (SweepResult :type Hit%20Result%20Structure%20%28by%20ref%29))
  (Utilities|Casting|CastToCH_Player OtherActor)
  (Variables|Default|SetinRange true))

(event OnComponentEndOverlap(Collision)
  (params (OverlappedComponent :type Primitive%20Component%20Object%20Reference) (OtherActor :type Actor%20Object%20Reference) (OtherComp :type Primitive%20Component%20Object%20Reference) (OtherBodyIndex :type Integer))
  (Utilities|Casting|CastToCH_Player OtherActor)
  (Variables|Default|SetinRange false))

(event EventBeginPlay)

(event Collision|EventActorBeginOverlap
  (params (OtherActor :type Actor%20Object%20Reference)))

(event EventTick
  (params (DeltaSeconds :type Float%20%28single-precision%29)))

(event EventBeingPickedUp
  (params (Instigator :type Actor%20Object%20Reference))
  (bind _aspc_player (Utilities|Casting|CastToPC_Player Instigator))
  (Utilities|Array|Add (Variables|/Game/project_a/Blueprints/Core/PC_Player.PC_Player_C|GetInventory _aspc_player) (Variables|Default|GetItemInformation))
  (Actor|DestroyActor))

(fn ConstructionScript)