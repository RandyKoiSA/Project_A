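; Base world item pickup that holds item information and pops up with a random linear impulse plus a spin on spawn.
; Collision overlap with CH_Player toggles an InRange flag.
; BeingPickedUp adds the item to PC_Player's inventory component, then either destroys the actor or pops it again and stores the returned item information.
; SetMaxQuantityDrop randomizes the quantity between one and a given maximum.
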(event OnComponentBeginOverlap(Collision)
  (params (OverlappedComponent :type Primitive%20Component%20Object%20Reference) (OtherActor :type Actor%20Object%20Reference) (OtherComp :type Primitive%20Component%20Object%20Reference) (OtherBodyIndex :type Integer) (bFromSweep :type Boolean) (SweepResult :type Hit%20Result%20Structure%20%28by%20ref%29))
  (Utilities|Casting|CastToCH_Player OtherActor)
  (Variables|Default|SetinRange true))

(event OnComponentEndOverlap(Collision)
  (params (OverlappedComponent :type Primitive%20Component%20Object%20Reference) (OtherActor :type Actor%20Object%20Reference) (OtherComp :type Primitive%20Component%20Object%20Reference) (OtherBodyIndex :type Integer))
  (Utilities|Casting|CastToCH_Player OtherActor)
  (Variables|Default|SetinRange false))

(event EventBeginPlay
  ;[1 1 1] Add impulse to object
  (CallFunction|PopItem))

(event Collision|EventActorBeginOverlap
  (params (OtherActor :type Actor%20Object%20Reference)))

(event EventTick
  (params (DeltaSeconds :type Float%20%28single-precision%29)))

(event EventBeingPickedUp
  (params (Instigator :type Actor%20Object%20Reference))
  ;[1 1 1] Pickup Item
  (bind _aspc_player (Utilities|Casting|CastToPC_Player (Game|GetPlayerController 0)))
  (bind (_bisnomoreitem _pickedupitem) (Default|AddItem (Variables|/Game/project_a/Blueprints/Core/PC_Player.PC_Player_C|GetBP_InventoryComponent _aspc_player) (Variables|Item|GetItemInformation)))
  (if _bisnomoreitem
    (Actor|DestroyActor)
    (else
      (CallFunction|PopItem)
      (Variables|Item|SetItemInformation _pickedupitem))))

(fn ConstructionScript)

(fn PopItem
  (bind _materialmesh (Variables|Default|GetMaterialMesh))
  (Physics|AddImpulse _materialmesh (Math|Vector|MakeVector (Math|Random|RandomFloatinRange 0.0 3e+02) (Math|Random|RandomFloatinRange 0.0 3e+02) 5e+02) "None" false)
  (Class|PrimitiveComponent|AddAngularImpulseinDegrees _materialmesh "300.000000,300.000000,100.000000" "None" true))

(fn SetMaxQuantityDrop
  (params (MaxQuantityChance :type Integer))
  (bind _output_get (LocalVariables|SetMaxQuant MaxQuantityChance))
  (Variables|Item|SetItemInformation (Utilities|Struct|MakeS_Item (.name (Variables|Item|GetItemInformation)) (.description (Variables|Item|GetItemInformation)) (.icon (Variables|Item|GetItemInformation)) (.category (Variables|Item|GetItemInformation)) (Math|Random|RandomIntegerinRange 1 _output_get) (.maxquantity (Variables|Item|GetItemInformation)))))