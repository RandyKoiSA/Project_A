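; Player HUD that builds the main on-screen UI and manages a timed progress bar.
; On BeginPlay it adds WBP_HUD to the viewport, then anchors a status widget top-center and a hot bar bottom-center on its canvas, and caches the PC_Player controller.
; CreateProgressBar lazily creates the progress widget, sets its times and displays it directly in the viewport.
; ShowProgressBar toggles its visibility, returning whether the widget existed.
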(event EventBeginPlay
  (Utilities|FlowControl|Sequence
    (:then_0
      ;[0.2599 0.04416 1] Create HUD display
      (Utilities|IsValid (Variables|Default|GetHUD%20widget%20reference)
        (:Is%20Valid
          _)
        (:Is%20Not%20Valid
          (bind _returnvalue (UserInterface|CreateWidget "/Game/project_a/Blueprints/Widgets/WBP_HUD.WBP_HUD_C" (Game|GetPlayerController 0)))
          (bind _output_get (Variables|Default|SetHUD%20widget%20reference _returnvalue))))
      (UserInterface|Viewport|AddtoViewport _output_get 0))
    (:then_1
      ;[1 1 1] Create Status
      (Utilities|IsValid (Variables|Default|GetStatusRef)
        (:Is%20Valid
          _)
        (:Is%20Not%20Valid
          (bind _returnvalue_2 (UserInterface|CreateWidget "/Game/project_a/Blueprints/Widgets/WBP_Status.WBP_Status_C" (Game|GetPlayerController 0)))
          (bind _output_get_2 (Variables|Default|SetStatusRef _returnvalue_2))))
      (bind _returnvalue_3 (Class|CanvasPanel|AddChildtoCanvas (Variables|/Game/project_a/Blueprints/Widgets/WBP_HUD.WBP_HUD_C|GetHUD_canvas (Variables|Default|GetHUD%20widget%20reference)) _output_get_2))
      (Class|CanvasPanelSlot|SetAutoSize _returnvalue_3 true)
      (Class|CanvasPanelSlot|SetAnchors _returnvalue_3 (Utilities|Struct|MakeAnchors "(X=0.500000,Y=0.000000)" "(X=0.500000,Y=0.000000)"))
      (Class|CanvasPanelSlot|SetAlignment _returnvalue_3 "(X=0.500000,Y=0.000000)")
      (Class|CanvasPanelSlot|SetPosition _returnvalue_3 "(X=0.000000,Y=10.000000)"))
    (:then_2
      ;[1 1 1] Get Player Controller
      (bind _aspc_player (Utilities|Casting|CastToPC_Player (Game|GetPlayerController 0)))
      (Variables|Default|SetPlayerControllerRef _aspc_player))
    (:then_3
      ;[1 1 1] Add Hot Bar
      (bind _returnvalue_4 (UserInterface|CreateWidget "/Game/project_a/Blueprints/Widgets/Inventory/WBP_HotBar.WBP_HotBar_C" (Game|GetPlayerController 0)))
      (bind _output_get_3 (Variables|Default|SetHotBar%20REF _returnvalue_4))
      (bind _returnvalue_5 (Class|CanvasPanel|AddChildtoCanvas (Variables|/Game/project_a/Blueprints/Widgets/WBP_HUD.WBP_HUD_C|GetHUD_canvas (Variables|Default|GetHUD%20widget%20reference)) _output_get_3))
      (Class|CanvasPanelSlot|SetAutoSize _returnvalue_5 true)
      (Class|CanvasPanelSlot|SetAnchors _returnvalue_5 (Utilities|Struct|MakeAnchors "(X=0.500000,Y=1.000000)" "(X=0.500000,Y=1.000000)"))
      (Class|CanvasPanelSlot|SetAlignment _returnvalue_5 "(X=0.500000,Y=1.100000)"))))

(fn ConstructionScript)

(fn CreateProgressBar
  (params (MaxTime :type Float%20%28single-precision%29) (CurrentTime :type Float%20%28single-precision%29))
  (Utilities|IsValid (Variables|Default|GetProgressBarRef)
    (:Is%20Valid
      _)
    (:Is%20Not%20Valid
      (bind _returnvalue (UserInterface|CreateWidget "/Game/project_a/Blueprints/Widgets/WBP_Progress.WBP_Progress_C" (Game|GetPlayerController 0)))
      (bind _output_get (Variables|Default|SetProgressBarRef _returnvalue))))
  (Variables|/Game/project_a/Blueprints/Widgets/WBP_Progress.WBP_Progress_C|SetMaxTime _output_get MaxTime)
  (Variables|/Game/project_a/Blueprints/Widgets/WBP_Progress.WBP_Progress_C|SetCurrentTime _output_get CurrentTime)
  (UserInterface|Viewport|AddtoViewport _output_get 0)
  (Widget|SetVisibility _output_get "Visible"))

(fn ShowProgressBar
  (params (Show? :type Boolean))
  (bind _progressbarref (Variables|Default|GetProgressBarRef))
  (if Show?
    (Utilities|IsValid _progressbarref
      (:Is%20Valid
        (Widget|SetVisibility _progressbarref "Visible")
        (return true))
      (:Is%20Not%20Valid
        (return false)))
    (else
      (Utilities|IsValid _progressbarref
        (:Is%20Valid
          (Widget|SetVisibility _progressbarref "Hidden")
          (return true))
        (:Is%20Not%20Valid
          (Development|PrintString "Can't display progress bar")
          (return false))))))