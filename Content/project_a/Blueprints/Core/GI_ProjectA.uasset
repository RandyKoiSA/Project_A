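; GI_ProjectA is a Game Instance Blueprint that holds the player inventory and adds picked-up items to it.
; AddItem merges the pickup into matching, non-full stacks by name, capping each at its max quantity and carrying overflow forward.
; Any remainder takes a new slot if space allows, and the function returns whether everything was taken plus any leftover item.
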(fn AddItem
  (params (Item :type S%20Item%20Structure))
  (LocalVariables|SetPickupItem Item)
  ;[1 1 1] Check if any space in inventory
  (if (<= (Utilities|Array|Length (Variables|Default|GetInventory)) (Variables|Default|GetMaxInventorySpace))
    (bind (_array_element _array_index) (Utilities|Array|ForEachLoopwithBreak (Variables|Default|GetInventory) :!label _label)
      (:LoopBody
        (LocalVariables|SetInventoryItem _array_element)
        ;[1 1 1] Check if  there is still space
        (LocalVariables|SetcurrentIndex _array_index)
        (if (or (> (.quantity (LocalVariables|GetPickupItem)) 0) (< (Utilities|Array|Length (Variables|Default|GetInventory)) (Variables|Default|GetMaxInventorySpace)))
          ;[1 1 1] Check if the item is the same
          (if (Utilities|Enum|Equal(Enum) (.name (LocalVariables|GetInventoryItem)) (.name (LocalVariables|GetPickupItem)))
            ;[1 1 1] Check if max stacked
            (if (< (.quantity (LocalVariables|GetInventoryItem)) (.maxquantity (LocalVariables|GetInventoryItem)))
              ;[1 1 1] Add Item to Stack
              (Utilities|Array|SetArrayElem (Variables|Default|GetInventory) (LocalVariables|GetcurrentIndex) (Utilities|Struct|MakeS_Item (.name (LocalVariables|GetInventoryItem)) (.description (LocalVariables|GetInventoryItem)) (.icon (LocalVariables|GetInventoryItem)) (.category (LocalVariables|GetInventoryItem)) (+ (.quantity (LocalVariables|GetInventoryItem)) (.quantity (LocalVariables|GetPickupItem))) (.maxquantity (LocalVariables|GetInventoryItem))))
              ;[1 1 1] Check if stack is overflow
              (if (> (.Quantity (Utilities|Struct|BreakS_Item (Utilities|Array|Get(acopy) (Variables|Default|GetInventory) (LocalVariables|GetcurrentIndex)))) (.MaxQuantity (Utilities|Struct|BreakS_Item (Utilities|Array|Get(acopy) (Variables|Default|GetInventory) (LocalVariables|GetcurrentIndex)))))
                ;[1 1 1] Set Item Slot to Max Quantity
                (LocalVariables|SetLeftOver (- (.Quantity (Utilities|Struct|BreakS_Item (Utilities|Array|Get(acopy) (Variables|Default|GetInventory) (LocalVariables|GetcurrentIndex)))) (.MaxQuantity (Utilities|Struct|BreakS_Item (Utilities|Array|Get(acopy) (Variables|Default|GetInventory) (LocalVariables|GetcurrentIndex))))))
                (Utilities|Array|SetArrayElem (Variables|Default|GetInventory) (LocalVariables|GetcurrentIndex) (Utilities|Struct|MakeS_Item (.Name (Utilities|Struct|BreakS_Item (Utilities|Array|Get(acopy) (Variables|Default|GetInventory) (LocalVariables|GetcurrentIndex)))) (.Description (Utilities|Struct|BreakS_Item (Utilities|Array|Get(acopy) (Variables|Default|GetInventory) (LocalVariables|GetcurrentIndex)))) (.Icon (Utilities|Struct|BreakS_Item (Utilities|Array|Get(acopy) (Variables|Default|GetInventory) (LocalVariables|GetcurrentIndex)))) (.Category (Utilities|Struct|BreakS_Item (Utilities|Array|Get(acopy) (Variables|Default|GetInventory) (LocalVariables|GetcurrentIndex)))) (.MaxQuantity (Utilities|Struct|BreakS_Item (Utilities|Array|Get(acopy) (Variables|Default|GetInventory) (LocalVariables|GetcurrentIndex)))) (.MaxQuantity (Utilities|Struct|BreakS_Item (Utilities|Array|Get(acopy) (Variables|Default|GetInventory) (LocalVariables|GetcurrentIndex))))))
                ;[1 1 1] Set leftover quantity back to pickup item
                (LocalVariables|SetPickupItem (Utilities|Struct|MakeS_Item (.name (LocalVariables|GetPickupItem)) (.description (LocalVariables|GetPickupItem)) (.icon (LocalVariables|GetPickupItem)) (.category (LocalVariables|GetPickupItem)) (LocalVariables|GetLeftOver) (.maxquantity (LocalVariables|GetPickupItem))))
                (else
                  ;[1 1 1] Set pickup item quantity to zero
                  (LocalVariables|SetPickupItem (Utilities|Struct|MakeS_Item (.name (LocalVariables|GetPickupItem)) (.description (LocalVariables|GetPickupItem)) (.icon (LocalVariables|GetPickupItem)) (.category (LocalVariables|GetPickupItem)) 0 (.maxquantity (LocalVariables|GetPickupItem))))
                  (goto _label Break)))))
          (else
            (goto _label Break))))
      (:Completed
        ;[1 1 1] Completed Loop
        ;;[1 1 1] Check if there is any items left
        (if (> (.quantity (LocalVariables|GetPickupItem)) 0)
          ;;[1 1 1 1 10] Check if there is still inventory room
          (if (< (Utilities|Array|Length (Variables|Default|GetInventory)) (Variables|Default|GetMaxInventorySpace))
            ;;[1 1 1] Add Item to inventory
            (Utilities|Array|Add (Variables|Default|GetInventory) (LocalVariables|GetPickupItem))
            (return true (LocalVariables|GetPickupItem))
            (else
              ;;[1 1 1] Return leftover items back
              (return false (LocalVariables|GetPickupItem))))
          (else
            (return true (LocalVariables|GetPickupItem))))))
    (else
      (return false (LocalVariables|GetPickupItem)))))