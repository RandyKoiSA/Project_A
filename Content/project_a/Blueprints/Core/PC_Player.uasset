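; PC_Player is the player controller that handles shooting, interaction and item pickup input for the player character.
; Action spawns BP_Bullet at the character, rotated toward the hit under the cursor.
; Interact and Pickup message the first capsule-overlapping actor implementing I_Interact or I_Pickup, with Interact also tracking held state and messaging again on release.
; BeginPlay caches GI_ProjectA, whose inventory quantities a debug key prints.
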(event EventBeginPlay
  ;[1 1 1] Begin Play
  (Utilities|FlowControl|Sequence
    (:then_0
      (bind _asgi_project_a (Utilities|Casting|CastToGI_ProjectA (Game|GetGameInstance)))
      (Variables|Default|SetGameInstanceREF _asgi_project_a))))

(event Input|ActionEvents|InputActionPickup
  (params (Key :type Key%20Structure :default "None"))
  ;[1 1 1] Pickup
  (:Pressed
    (bind _array_element (Utilities|Array|ForEachLoopwithBreak (Collision|GetOverlappingActors (Variables|/Script/Engine.Character|GetCapsuleComponent (Game|GetPlayerCharacter 0)) 0 :!class /Script/Engine.PrimitiveComponent) :!label _label)
      (:LoopBody
        (if (Utilities|DoesObjectImplementInterface _array_element "/Game/project_a/Blueprints/Interfaces/I_Pickup.I_Pickup_C")
          (bind _output_get (Variables|Default|SetPickupObject _array_element))
          (Class|IPickup|BeingPickedUp(Message) _output_get self)
          (goto _label Break))))))

(event Input|ActionEvents|InputActionInteract
  (params (Key :type Key%20Structure :default "None"))
  ;[1 1 1] Interaction Key
  (:Pressed
    (Variables|Default|SetisInteracting true)
    (bind _array_element (Utilities|Array|ForEachLoopwithBreak (Collision|GetOverlappingActors (Variables|/Script/Engine.Character|GetCapsuleComponent (Game|GetPlayerCharacter 0)) 0 :!class /Script/Engine.PrimitiveComponent) :!label _label)
      (:LoopBody
        (if (Utilities|DoesObjectImplementInterface _array_element "/Game/project_a/Blueprints/Interfaces/I_Interact.I_Interact_C")
          (bind _output_get (Variables|Default|SetInterableObject _array_element))
          (Class|IInteract|BeingInteracted(Message) _output_get)
          (goto _label Break)))))
  (:Released
    (Variables|Default|SetisInteracting false)
    (Utilities|IsValid (Variables|Default|GetInterableObject)
      (:Is%20Valid
        (Class|IInteract|BeingInteracted(Message) (Variables|Default|GetInterableObject))))))

(event Input|ActionEvents|InputActionAction
  (params (Key :type Key%20Structure :default "None"))
  (bind _returnvalue (Game|GetPlayerCharacter 0))
  (bind _returnvalue_2 (Transformation|GetActorTransform _returnvalue))
  (bind _location (Math|Transform|BreakTransform _returnvalue_2))
  ;[1 1 1] Action Key
  (:Pressed
    (Game|SpawnActorfromClass "/Game/project_a/Blueprints/BP_Bullet.BP_Bullet_C" (Math|Transform|MakeTransform _location (Math|Rotator|FindLookatRotation _location (.Location (Collision|BreakHitResult (.HitResult (Game|Player|GetHitResultUnderCursorbyChannel "TraceTypeQuery1" true))))) "1,1,1") "Undefined" 0 0)))

(event Input|KeyboardEvents|1
  (params (Key :type Key%20Structure :default "None"))
  (:Pressed
    (for _array_element (Variables|/Game/project_a/Blueprints/Core/GI_ProjectA.GI_ProjectA_C|GetInventory (Variables|Default|GetGameInstanceREF))
      (Development|PrintString (Utilities|String|ToString(Integer) (.Quantity (Utilities|Struct|BreakS_Item _array_element)))))))

(fn ConstructionScript)