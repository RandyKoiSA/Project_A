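; Inventory component that adds picked-up items to a slot array, stacking them by name.
; AddItem merges the pickup into the first same-name slot with space, otherwise appends a new slot if under MaxSlots.
; It returns a completion flag and the remaining item, rebuilding structs with a hardcoded cube mesh.
; The overflow check reads the pre-merge quantity, so stacks can exceed MaxQuantity without producing leftovers.
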(event EventBeginPlay)

(event EventTick
  (params (DeltaSeconds :type Float%20%28single-precision%29)))

(fn AddItem
  (params (ItemInfo :type S%20Item%20Structure))
  (bind _inventory (Variables|Default|GetInventory))
  (LocalVariables|SetPick%20Up%20Item ItemInfo)
  (for (_array_element _array_index) (.inventoryslots (Variables|Default|GetInventory))
    (LocalVariables|SetItem _array_element)
    (LocalVariables|SetIndex _array_index)
    ;[1 1 1] Check if there any more items left to put in inventory
    (if (> (.quantity (LocalVariables|GetPick%20Up%20Item)) 0)
      ;[1 1 1] Check if Item Name are the Same
      (if (Utilities|Enum|Equal(Enum) (.name (LocalVariables|GetItem)) (.name (LocalVariables|GetPick%20Up%20Item)))
        ;[1 1 1] Check if there is space in the slot
        (if (< (.quantity (LocalVariables|GetItem)) (.maxquantity (LocalVariables|GetItem)))
          ;[1 1 1] Add pickup item quantity to item quantity
          (Utilities|Array|SetArrayElem (.inventoryslots (Variables|Default|GetInventory)) (LocalVariables|GetIndex) (Utilities|Struct|MakeS_Item (.name (LocalVariables|GetItem)) (.description (LocalVariables|GetItem)) (.icon (LocalVariables|GetItem)) (.category (LocalVariables|GetItem)) (+ (.quantity (LocalVariables|GetItem)) (.quantity (LocalVariables|GetPick%20Up%20Item))) (.maxquantity (LocalVariables|GetItem)) 0 "/Game/Geometry/Meshes/1M_Cube.1M_Cube"))
          ;[1 1 1] Set Pickup Quantity To Zero
          (LocalVariables|SetPick%20Up%20Item (Utilities|Struct|MakeS_Item (.name (LocalVariables|GetPick%20Up%20Item)) (.description (LocalVariables|GetPick%20Up%20Item)) (.icon (LocalVariables|GetPick%20Up%20Item)) (.category (LocalVariables|GetPick%20Up%20Item)) 0 (.maxquantity (LocalVariables|GetPick%20Up%20Item)) 0 "/Game/Geometry/Meshes/1M_Cube.1M_Cube"))
          ;[1 1 1] Check if the item quantity is overloaded
          (if (> (.quantity (LocalVariables|GetItem)) (.maxquantity (LocalVariables|GetItem)))
            ;[1 1 1] Set Pickup Item Quantity the leftover
            (LocalVariables|SetPick%20Up%20Item (Utilities|Struct|MakeS_Item (.name (LocalVariables|GetPick%20Up%20Item)) (.description (LocalVariables|GetPick%20Up%20Item)) (.icon (LocalVariables|GetPick%20Up%20Item)) (.category (LocalVariables|GetPick%20Up%20Item)) (- (.quantity (LocalVariables|GetItem)) (.maxquantity (LocalVariables|GetItem))) (.maxquantity (LocalVariables|GetPick%20Up%20Item)) 0 "/Game/Geometry/Meshes/1M_Cube.1M_Cube"))
            (else
              (Development|PrintString "COMPLETE: BREAK" false)
              (return true (Utilities|Struct|MakeS_Item (.name (LocalVariables|GetPick%20Up%20Item)) (.description (LocalVariables|GetPick%20Up%20Item)) (.icon (LocalVariables|GetPick%20Up%20Item)) (.category (LocalVariables|GetPick%20Up%20Item)) 0 (.maxquantity (LocalVariables|GetPick%20Up%20Item)) 0 "/Game/Geometry/Meshes/1M_Cube.1M_Cube"))))
          (else
            (Development|PrintString "The Item slot is maxed out. Go to next item" false)))
        (else
          (Development|PrintString "This item is not the same as the pick up item. Go to next item" false)))
      (else
        (Development|PrintString "No more items to put in" false))))
  ;[0.1978 0.2996 1] Completed
  ;;[1 1 1] Check if there is any item quantity left
  (if (> (.quantity (LocalVariables|GetPick%20Up%20Item)) 0)
    ;;[1 1 1] Check if there is still inventory space
    (if (< (Utilities|Array|Length (.inventoryslots _inventory)) (.maxslots _inventory))
      ;;[1 1 1] Add Item to inventory
      (Utilities|Array|Add (.inventoryslots (Variables|Default|GetInventory)) (LocalVariables|GetPick%20Up%20Item))
      (return true (Utilities|Struct|MakeS_Item (.name (LocalVariables|GetPick%20Up%20Item)) (.description (LocalVariables|GetPick%20Up%20Item)) (.icon (LocalVariables|GetPick%20Up%20Item)) (.category (LocalVariables|GetPick%20Up%20Item)) 0 (.maxquantity (LocalVariables|GetPick%20Up%20Item)) 0 "/Game/Geometry/Meshes/1M_Cube.1M_Cube"))
      (else
        ;;[1 1 1] Return leftover items back
        (return false (LocalVariables|GetPick%20Up%20Item))))
    (else
      ;;[1 1 1] No more items
      (return true (LocalVariables|GetPick%20Up%20Item)))))